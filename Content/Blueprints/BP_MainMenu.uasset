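; BP_MainMenu handles player input setup, a narrow camera yaw limit and the pause toggle, going by its name for the main menu.
; On BeginPlay it adds the IMC_Player mapping context and clamps the player camera manager's view yaw to a small range around zero.
; IA_Menu calls PauseGame or UnpauseGame on GM_Glühweinnachten, depending on the current pause state.
; An AddPoints call on GI_GW is left unconnected and never runs.
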(event Custom|SetupInputs
  (Input|AddMappingContext (PlayerController|LocalPlayerSubsystems|GetEnhancedInputLocalPlayerSubsystem (Game|GetPlayerController 0)) "/Game/Blueprints/IMC_Player.IMC_Player" 0 "(bIgnoreAllPressedKeysUntilRelease=True,bForceImmediately=False)"))

(event Custom|YawClamp
  (bind _returnvalue (Game|GetPlayerCameraManager 0))
  (Variables|/Script/Engine.PlayerCameraManager|SetViewYawMin _returnvalue -7.5)
  (Variables|/Script/Engine.PlayerCameraManager|SetViewYawMax _returnvalue 7.5))

(event Input|EnhancedActionEvents|EnhancedInputActionIA_Menu
  (params (ActionValue :type Boolean) (ElapsedSeconds :type Float%20%28double-precision%29) (TriggeredSeconds :type Float%20%28double-precision%29) (InputAction :type Input%20Action%20Object%20Reference :default "/Game/Blueprints/IA_Menu.IA_Menu"))
  (:Triggered
    (bind _asgm_glühweinnachten (Utilities|Casting|CastToGM_Glühweinnachten (Game|GetGameMode)))
    (if (Game|IsGamePaused)
      (Default|UnpauseGame _asgm_glühweinnachten)
      (else
        (Default|PauseGame _asgm_glühweinnachten)))))

(event EventBeginPlay
  (CallFunction|SetupInputs)
  (CallFunction|YawClamp))

(event Collision|EventActorBeginOverlap
  (params (OtherActor :type Actor%20Object%20Reference)))

(event EventTick
  (params (DeltaSeconds :type Float%20%28single-precision%29)))

(fn ConstructionScript)