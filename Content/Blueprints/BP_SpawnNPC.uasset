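; BP_SpawnNPC is an actor that drives a ChildActor component to place a BP_NPC at randomized positions.
; BeginPlay caches the first BP_NPC found, then every five seconds sets the child class and randomizes its relative X and Z offset.
; The random class pick has BP_NPC in both options, so the class never varies.
; An uncalled Clock event would poll the cached NPC's IsClicked flag and clear it.
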(event Custom|Clock
  (bind _newvar (Variables|Default|GetNewVar))
  (if (Variables|/Game/Blueprints/BP_NPC.BP_NPC_C|GetIsClicked? _newvar) :!label _label
    (Variables|/Game/Blueprints/BP_NPC.BP_NPC_C|SetIsClicked? _newvar false)
    (else
      (Utilities|FlowControl|Delay 3.0)
      (goto _label))))

(event EventBeginPlay
  (bind _returnvalue (Math|Random|RandomFloatinRange -2.5 2.5))
  (bind _outactors (Actor|GetAllActorsOfClass "/Game/Blueprints/BP_NPC.BP_NPC_C"))
  (Variables|Default|SetNewVar (Utilities|Array|Get(acopy) _outactors))
  (ChildActorComponent|SetChildActorClass (Variables|Default|GetChildActor) (Utilities|Select :Index (Math|Random|RandomIntegerinRange 0 1) :Option%200 "/Game/Blueprints/BP_NPC.BP_NPC_C" :Option%201 "/Game/Blueprints/BP_NPC.BP_NPC_C") :!label _label)
  (Transformation|SetRelativeLocation (Variables|Default|GetChildActor) (Math|Vector|MakeVector _returnvalue 0.0 _returnvalue) false false)
  (Utilities|FlowControl|Delay 5.0)
  (goto _label))

(fn ConstructionScript)