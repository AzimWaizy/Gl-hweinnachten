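; BP_NPC is a clickable customer-style NPC that shows one of six random animal materials on its plane.
; On BeginPlay it binds its click event and caches the first BP_Kessel (cauldron) in the level.
; A click plays a sound, destroys BP_Tasse (cup) actors and re-enables cauldron spawning.
; If the cauldron's IsSpawned flag is set, it awards points through the GI_GW game instance and clears the flag.
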(event Custom|OnMouseClicked
  (params (TouchedActor :type Actor%20Object%20Reference) (ButtonPressed :type Key%20Structure :default "None"))
  (bind _kesselref (Variables|Default|GetKesselRef))
  (Audio|PlaySound2D "/Game/Sound/Sound/InGame/Neues_Rezept_erscheint.Neues_Rezept_erscheint" 1.0 1.0 0.0 0 0)
  (Variables|Default|SetIsClicked? true)
  (bind _outactors (Actor|GetAllActorsOfClass "/Game/Blueprints/BP_Tasse.BP_Tasse_C"))
  (Actor|DestroyActor _outactors)
  (Variables|/Game/Blueprints/BP_Kessel.BP_Kessel_C|SetCanSpawn? _kesselref true)
  (if (Variables|/Game/Blueprints/BP_Kessel.BP_Kessel_C|GetIsSpawned _kesselref)
    (bind _asgi_gw (Utilities|Casting|CastToGI_GW (Game|GetGameInstance)))
    (Default|AddPoints _asgi_gw 50)
    (Variables|/Game/Blueprints/BP_Kessel.BP_Kessel_C|SetIsSpawned _kesselref false)))

(event EventBeginPlay
  (Utilities|FlowControl|Sequence
    (:then_0
      (EventDispatchers|BindEventtoOnClicked (delegate Custom|OnMouseClicked)))
    (:then_1
      (bind _outactors (Actor|GetAllActorsOfClass "/Game/Blueprints/BP_Kessel.BP_Kessel_C"))
      (Variables|Default|SetKesselRef (Utilities|Array|Get(acopy) _outactors)))
    (:then_2
      (Rendering|Material|SetMaterial (Variables|Default|GetPlane) 0 (Utilities|Select :Index (Math|Random|RandomIntegerinRange 0 5) :Option%200 "/Game/Assets/Chars/Mi_Axolottle.Mi_Axolottle" :Option%201 "/Game/Assets/Chars/Mi_Bear.Mi_Bear" :Option%202 "/Game/Assets/Chars/Mi_Elefant.Mi_Elefant" :Option%203 "/Game/Assets/Chars/Mi_Hai.Mi_Hai" :Option%204 "/Game/Assets/Chars/Mi_Kroko.Mi_Kroko" :Option%205 "/Game/Assets/Chars/Mi_Wale.Mi_Wale")))))

(fn ConstructionScript)